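; HUD for the quest system that creates and displays the main UI and dialog widgets at BeginPlay.
; Toggles the full-screen quest list in the main UI, re-initializing it each time a hidden list is shown.
; Spawns a quest description widget on the main canvas, anchored near the top right, skipping empty or placeholder text, and removes it on hide.
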(event `self.ReceiveBeginPlay`
  (bind _returnvalue (`|CreateWidget` "/Game/UI/W_Main.W_Main_C" (`GameplayStatics.GetPlayerController` 0)))
  (bind _output_get (set `self.MainUI` _returnvalue))
  (`UserWidget.AddToViewport` _output_get 0)
  (bind _returnvalue_2 (`|CreateWidget` "/DialogPlugin/DialogPlugin/UI/WBP_MainDialog.WBP_MainDialog_C" (`GameplayStatics.GetPlayerController` 0)))
  (bind _output_get_2 (set `self.DialogUI` _returnvalue_2))
  (`UserWidget.AddToViewport` _output_get_2 0))

(event `ToggleQuestList`
  (bind _w_fullscreenquestlist (`/Game/UI/W_Main.W_FullScreenQuestList` (`self.MainUI`)))
  (switch `ESlateVisibility` (`Widget.Visibility` _w_fullscreenquestlist)
    (:`Visible`
      (`Widget.SetVisibility` _w_fullscreenquestlist "Hidden"))
    (:`Hidden`
      (`/Game/UI/W_FullScreenQuestList.Initialzie` _w_fullscreenquestlist)
      (`Widget.SetVisibility` _w_fullscreenquestlist "Visible"))))

(event `ShowQuestDescription`
  (params (QuestInfo :type "QuestInfo Object Reference"))
  (bind _description (`QuestInfo.Description` QuestInfo))
  (if (not (or (== _description "Description") (== _description "")))
    (bind _returnvalue (`|GenericCreateObject` "/Game/UI/W_QuestDescription.W_QuestDescription_C" _description))
    (bind _output_get (set `self.QuestDescription` _returnvalue))
    (bind _returnvalue_2 (`CanvasPanel.AddChildToCanvas` (`/Game/UI/W_Main.CanvasPanel_29` (`self.MainUI`)) _output_get))
    (`CanvasPanelSlot.SetAnchors` _returnvalue_2 (make `Anchors` (1.0 0.145) (1.0 0.145)))
    (`CanvasPanelSlot.SetPosition` _returnvalue_2 (-50.0 0.0))
    (`CanvasPanelSlot.SetAlignment` _returnvalue_2 (1.0 0.0))
    (`CanvasPanelSlot.SetSize` _returnvalue_2 (500.0 500.0))))

(event `HideQuestDescription`
  (bind _questdescription (`self.QuestDescription`)
    (:`then`
      (`Widget.RemoveFromParent` _questdescription)
      (set `self.QuestDescription` null))
    (:`else`)))

(fn `UserConstructionScript`)