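; BP_NPC is an interactable NPC that hands quest content to the player's quest system.
; On Interact it prints the NPC's name for debugging, then adds its ChainQuest, if valid, to the QuestWorldSubsystem.
; It also always pushes its GameplayTags to that subsystem, so talking to the NPC can register tags with the quest system.
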(event `/Game/Blueprints/Npc/BPI_Interact.Interact`
  (`KismetSystemLibrary.PrintString` (`KismetTextLibrary.Conv_TextToString` (`|FormatText` "Interacted with NPC: {NPCName}" (`self.Name`))))
  (`/Engine/EditorBlueprintResources/StandardMacros.IsValid` (`self.ChainQuest`)
    (:`Is Valid`
      (`QuestWorldSubsystem.AddChainQuest` (subsystem `QuestWorldSubsystem`) (`self.ChainQuest`)))
    (:`Is Not Valid`
      _))
  (`QuestWorldSubsystem.AddGameplayTags` (subsystem `QuestWorldSubsystem`) (`self.Gameplay Tags`)))

(fn `UserConstructionScript`)